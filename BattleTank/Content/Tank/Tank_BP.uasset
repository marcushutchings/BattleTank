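; Player tank pawn Blueprint that routes input to track, aiming and firing components.
; On BeginPlay it hands both tracks to the TankMovement component, then supports direct per-track throttle axes or intent-based forward and turn input through that component.
; Aim axes rotate separate azimuth and elevation gimbals, scaled by frame delta time, and the Fire action calls the TankAiming component.
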(event EventBeginPlay
  (Class|TankMovementComponent|Initialise (Variables|Default|GetTankMovement) (Variables|Default|GetTrack%20Left) (Variables|Default|GetTrack%20Right)))

(event Input|ActionEvents|InputActionFire
  (params (Key :type Key%20Structure))
  ;[1 1 1] Aim Control
  (:Pressed
    (Class|TankAimingComponent|Fire (Variables|Default|GetTankAiming))))

(event Input|AxisEvents|InputAxisAimAzimuth
  (params (AxisValue :type Float%20%28single-precision%29))
  ;[1 1 1] Aim Control
  (Transformation|AddLocalRotation (Variables|Default|GetAzimuth_Gimble) (Math|Rotator|MakeRotator 0.0 0.0 (* AxisValue (Utilities|Time|GetWorldDeltaSeconds) 1e+02)) false false))

(event Input|AxisEvents|InputAxisLeftTrackThrottle
  (params (AxisValue :type Float%20%28single-precision%29))
  ;[1 1 1] Input Movement Binding
  (Class|TankTrack|SetThrottle (Variables|Default|GetTrack%20Left) AxisValue))

(event Input|AxisEvents|InputAxisRightTrackThrottle
  (params (AxisValue :type Float%20%28single-precision%29))
  ;[1 1 1] Input Movement Binding
  (Class|TankTrack|SetThrottle (Variables|Default|GetTrack%20Right) AxisValue))

(event Input|AxisEvents|InputAxisIntendMoveRight
  (params (AxisValue :type Float%20%28single-precision%29))
  ;[1 1 1] Input Movement Binding
  (Class|TankMovementComponent|IntendTurnRight (Variables|Default|GetTankMovement) AxisValue))

(event Input|AxisEvents|InputAxisAimElevation
  (params (AxisValue :type Float%20%28single-precision%29))
  ;[1 1 1] Aim Control
  (Transformation|AddLocalRotation (Variables|Default|GetElevation_Gimble) (Math|Rotator|MakeRotator 0.0 (* AxisValue (Utilities|Time|GetWorldDeltaSeconds) 1e+02) 0.0) false false))

(event Input|AxisEvents|InputAxisIntendMoveForward
  (params (AxisValue :type Float%20%28single-precision%29))
  ;[1 1 1] Input Movement Binding
  (Class|TankMovementComponent|IntendMoveForward (Variables|Default|GetTankMovement) AxisValue))

(fn ConstructionScript)